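; BP_Player is the player character Blueprint, providing a melee combo attack through the Gameplay Ability System.
; Attack, when not falling, tries to activate GA_Melee, then advances ComboCount regardless of success, wrapping at the AttackMontages length.
; WeaponCapsule overlaps with other actors send a Skill.melee.dealDamage gameplay event to the player, carrying the hit actor as Target.
; Health changes are only printed to screen.
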(event `self.WeaponCapsule.OnComponentBeginOverlap`
  (params (OverlappedComponent :type "PrimitiveComponent Object Reference") (OtherActor :type "Actor Object Reference") (OtherComp :type "PrimitiveComponent Object Reference") (OtherBodyIndex :type Integer) (bFromSweep :type Boolean) (SweepResult :type "HitResult Structure (by ref)"))
  (if (!= OtherActor self)
    (`AbilitySystemBlueprintLibrary.SendGameplayEventToActor` self (struct :`TagName` "skill.melee.dealDamage") (make `GameplayEventData` (struct) null OtherActor))))

(event `self.K2_OnHealthChange`
  (params (Value :type "Float (single-precision)") (MaxValue :type "Float (single-precision)"))
  (`KismetSystemLibrary.PrintString` (`KismetStringLibrary.Conv_DoubleToString` Value)))

(fn `Attack`
  (if (not (`NavMovementComponent.IsFalling` (`self.CharacterMovement`)))
    (`AbilitySystemComponent.TryActivateAbilityByClass` (`self.AbilitySystemComp`) "/Game/Blueprints/GameplayAbilities/Melee/GA_Melee.GA_Melee_C" true)
    (bind _result (`/Engine/EditorBlueprintResources/StandardMacros.IncrementInt` (`self.ComboCount`))
      (:`  `
        (if (>= _result (`KismetArrayLibrary.Array_Length` (`self.AttackMontages`)))
          (set `self.ComboCount` 0))))))

(fn `UserConstructionScript`)