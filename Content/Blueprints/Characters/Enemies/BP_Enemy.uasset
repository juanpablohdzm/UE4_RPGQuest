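; Enemy character Blueprint that attacks through the Gameplay Ability System, can be stunned, and dies when its health runs out.
; Seeing the player writes it to the AI Blackboard and reveals the health bar widget.
; Health changes update that bar and, if dead, play a death montage and destroy the actor just before it ends.
; Stuns disable the controller and play a montage for a given time.
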(event `Attack`
  (`AbilitySystemComponent.TryActivateAbilityByClass` (`self.AbilitySystemComp`) (`self.AttackAbility`) true))

(event `Stunt`
  (params (Time :type "Float (double-precision)"))
  (set `self.IsStunted` true)
  (`self.DisableController`)
  (`self.PlayAnimMontage` (`self.StuntAnimMontage`))
  (`KismetSystemLibrary.Delay` Time)
  (`self.EnableController`)
  (`self.StopAnimMontage` (`self.StuntAnimMontage`))
  (set `self.IsStunted` false))

(event `self.K2_OnPawnSeen`
  (params (Pawn :type "Pawn Object Reference"))
  (bind _asbp_player (cast `/Game/Blueprints/Characters/Player/BP_Player` Pawn))
  (`BlackboardComponent.SetValueAsObject` (`AIBlueprintHelperLibrary.GetBlackboard` self) "Player" _asbp_player)
  (`SceneComponent.SetVisibility` (`self.HealthBar`) true false))

(event `self.K2_OnHealthChange`
  (params (Value :type "Float (single-precision)") (MaxValue :type "Float (single-precision)"))
  (bind _aswbp_enemy_health_bar (cast `/Game/UI/Widgets/WBP_EnemyHealthBar` (`WidgetComponent.GetUserWidgetObject` (`self.HealthBar`))))
  (`/Game/UI/Widgets/WBP_EnemyHealthBar.SetPercentage` _aswbp_enemy_health_bar (/ Value MaxValue))
  (if (`self.IsDead`)
    (bind _returnvalue (`self.PlayAnimMontage` (`self.DeadAnimMontage`)))
    (`KismetSystemLibrary.Delay` (- _returnvalue 0.2))
    (`self.K2_DestroyActor`)))

(fn `UserConstructionScript`)