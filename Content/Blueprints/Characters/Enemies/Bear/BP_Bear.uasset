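; BP_Bear is a bear enemy character driven by the BT_Enemy_Bear behavior tree and the Gameplay Ability System.
; On BeginPlay it acquires its attack ability and starts the tree through BP_AIController.
; When the left or right weapon collider overlaps a BP_Player, it sends itself a Bear.melee.damage gameplay event with that player as the target, leaving damage handling outside this graph.
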(event `self.ReceiveBeginPlay`
  (`self.AquireAbility` (`self.AttackAbility`))
  (bind _asbp_aicontroller (cast `/Game/Blueprints/Characters/Enemies/BP_AIController` (`AIBlueprintHelperLibrary.GetAIController` self)))
  (`AIController.RunBehaviorTree` _asbp_aicontroller "/Game/Blueprints/Characters/Enemies/Bear/BT_Enemy_Bear.BT_Enemy_Bear"))

(event `self.Weapon_L.OnComponentBeginOverlap`
  (params (OverlappedComponent :type "PrimitiveComponent Object Reference") (OtherActor :type "Actor Object Reference") (OtherComp :type "PrimitiveComponent Object Reference") (OtherBodyIndex :type Integer) (bFromSweep :type Boolean) (SweepResult :type "HitResult Structure (by ref)"))
  (if (!= OtherActor self)
    (cast `/Game/Blueprints/Characters/Player/BP_Player` OtherActor)
    (`AbilitySystemBlueprintLibrary.SendGameplayEventToActor` self (struct :`TagName` "bear.melee.damage") (make `GameplayEventData` (struct) null OtherActor))))

(event `self.Weapon_R.OnComponentBeginOverlap`
  (params (OverlappedComponent :type "PrimitiveComponent Object Reference") (OtherActor :type "Actor Object Reference") (OtherComp :type "PrimitiveComponent Object Reference") (OtherBodyIndex :type Integer) (bFromSweep :type Boolean) (SweepResult :type "HitResult Structure (by ref)"))
  (if (!= self OtherActor)
    (cast `/Game/Blueprints/Characters/Player/BP_Player` OtherActor)
    (`AbilitySystemBlueprintLibrary.SendGameplayEventToActor` self (struct :`TagName` "bear.melee.damage") (make `GameplayEventData` (struct) null OtherActor))))

(fn `UserConstructionScript`
  (`parent.UserConstructionScript`))