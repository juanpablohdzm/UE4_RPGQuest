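; BP_Grunt is a grunt enemy character that fights using gameplay abilities and an AI behavior tree.
; On BeginPlay it sets up health through its attribute set component, acquires attack and magic abilities, and runs BT_Enemy_Grunt on its AI controller.
; SetNextAbility uses a counter to switch the attack ability to an explosion every third call, otherwise melee.
; GetNextMontage alternates between two attack montages.
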(event `self.ReceiveBeginPlay`
  (bind _returnvalue (`self.GetAttributeSetComp`))
  (`RPGAttributeSet.ChangeHealthAmount` _returnvalue 300.0)
  (`self.AquireAbility` (`self.AttackAbility`))
  (`self.AquireAbility` (`self.MagicAbility`))
  (bind _asbp_aicontroller (cast `/Game/Blueprints/Characters/Enemies/BP_AIController` (`AIBlueprintHelperLibrary.GetAIController` self)))
  (`AIController.RunBehaviorTree` _asbp_aicontroller "/Game/Blueprints/Characters/Enemies/Grunt/BT_Enemy_Grunt.BT_Enemy_Grunt"))

(event `SetNextAbility`
  (bind _result (`/Engine/EditorBlueprintResources/StandardMacros.IncrementInt` (`self.AbilityCount`))
    (:`  `
      (if (== (mod _result 3) 0)
        (set `self.AttackAbility` "/Game/Blueprints/GameplayAbilities/Bear_Explosion/GA_Bear_Explosion.GA_Bear_Explosion_C")
        (else
          (set `self.AttackAbility` "/Game/Blueprints/GameplayAbilities/Bear_Melee/GA_Bear_Melee.GA_Bear_Melee_C"))))))

(fn `GetNextMontage`
  (returns (Montage :type "AnimMontage Object Reference"))
  (bind _result (`/Engine/EditorBlueprintResources/StandardMacros.IncrementInt` (`self.MontageIndex`))
    (:`  `
      (return (`|GetArrayItem` (`self.AttackMontages`) (mod _result 2))))))

(fn `UserConstructionScript`
  (`parent.UserConstructionScript`))