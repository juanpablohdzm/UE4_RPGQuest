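; GA_RPGBase is a base RPG gameplay ability that supplies a resource check and a player UI hook.
; CanActivateAbility gets the owner's attribute component and switches on cost type, adding the signed cost to mana or stamina and requiring a non-negative result.
; The health case ignores cost, only comparing base health to max health.
; PlayerActivateAbility casts through BP_Player to its controller to call ActivateUI; the activate and end events are empty.
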(fn `CanActivateAbility`
  (returns (Result :type Boolean))
  (locals (AttributeComp :type "RPGAttributeSet Object Reference"))
  (bind _attributecomp (`local.AttributeComp`))
  (bind (_stamina_basevalue _stamina_currentvalue) (break `GameplayAttributeData` (`RPGAttributeSet.Stamina` (`local.AttributeComp`))))
  (bind _health_basevalue (break `GameplayAttributeData` (`RPGAttributeSet.Health` _attributecomp)))
  (bind (_maxhealth_basevalue _maxhealth_currentvalue) (break `GameplayAttributeData` (`RPGAttributeSet.MaxHealth` _attributecomp)))
  (bind (_mana_basevalue _mana_currentvalue) (break `GameplayAttributeData` (`RPGAttributeSet.Mana` (`local.AttributeComp`))))
  (bind _returnvalue (message `RPGAttributeSetInterface.GetAttributeSetComp` (`self.GetOwningActorFromActorInfo`)))
  (bind _output_get (set `local.AttributeComp` _returnvalue))
  (`/Engine/EditorBlueprintResources/StandardMacros.IsValid` _output_get
    (:`Is Valid`
      (bind _returnvalue_2 (`self.GetAbilityInfo`))
      (switch `EAbilityCostType` (`.CostType` (break `GameplayAbilityInfo` _returnvalue_2))
        (:`HEALTH`
          (return (<= _health_basevalue _maxhealth_currentvalue)))
        (:`MANA`
          (return (>= (+ _mana_currentvalue (`.Cost` (break `GameplayAbilityInfo` _returnvalue_2))) 0.0)))
        (:`STAMINA`
          (return (>= (+ _stamina_currentvalue (`.Cost` (break `GameplayAbilityInfo` _returnvalue_2))) 0.0)))))
    (:`Is Not Valid`
      (`KismetSystemLibrary.PrintString` "IS not valid")
      (return false))))

(fn `PlayerActivateAbility`
  (bind _asbp_player (cast `/Game/Blueprints/Characters/Player/BP_Player` (`self.GetOwningActorFromActorInfo`)))
  (bind _asbp_player_controller (cast `/Game/Blueprints/BP_PlayerController` (`Pawn.GetController` _asbp_player)))
  (`/Game/Blueprints/BP_PlayerController.Activate UI` _asbp_player_controller))