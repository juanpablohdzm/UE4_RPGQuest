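; Gameplay ability for the Bear's explosion attack, which blasts players caught by its targeting actor.
; On activation it starts a user-confirmed target data wait with BP_BelowActor and plays the explosion montage after a short delay.
; Valid data spawns a large explosion effect, then launches each targeted player and applies a damage GameplayEffect.
; The ability ends with the montage, cancelling targeting and destroying the effect.
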(event `self.K2_ActivateAbility`
  (`self.K2_CommitAbility`)
  (bind (_asynctaskproxy _data) (`AbilityTask_WaitTargetData.WaitTargetData` "None" "UserConfirmed" "/Game/Blueprints/GameplayAbilities/Bear_Explosion/BP_BelowActor.BP_BelowActor_C" (struct) (struct) null)
    (:`then`
      (`KismetSystemLibrary.Delay` 0.3)
      (`AbilityTask_PlayMontageAndWait.CreatePlayMontageAndWaitProxy` "None" "/Game/Blueprints/Characters/Enemies/Bear/Animation/AM_Bear_Explosion.AM_Bear_Explosion"
        (:`OnCompleted`
          _)
        (:`OnBlendOut`
          _)
        (:`OnInterrupted`
          _)
        (:`OnCancelled`
          _))
      (`self.K2_EndAbility`))
    (:`ValidData`
      (bind _returnvalue (`GameplayStatics.SpawnEmitterAtLocation` "/Game/FXVarietyPack/Particles/P_ky_explosion.P_ky_explosion" (`AbilitySystemBlueprintLibrary.GetTargetDataEndPoint` _data (- (`AbilitySystemBlueprintLibrary.GetDataCountFromTargetData` _data) 1)) (struct) (7.0 7.0 7.0)))
      (set `self.PS` _returnvalue)
      (for _array_element (`AbilitySystemBlueprintLibrary.GetActorsFromTargetData` _data)
        (bind _asbp_player (cast `/Game/Blueprints/Characters/Player/BP_Player` _array_element))
        (bind _asbp_bear (cast `/Game/Blueprints/Characters/Enemies/Bear/BP_Bear` (`self.GetOwningActorFromActorInfo`)))
        (`RPGCharacter.PushCharacter` _asbp_bear _asbp_player 30.0 3000.0 true)
        (`self.BP_ApplyGameplayEffectToTarget` (`AbilitySystemBlueprintLibrary.AbilityTargetDataFromActor` _asbp_player) "/Game/Blueprints/GameplayAbilities/Bear_Explosion/Effect/GE_Bear_Explosion_Damage.GE_Bear_Explosion_Damage_C")))))

(event `self.K2_OnEndAbility`
  (params (bWasCancelled :type Boolean))
  (bind _ps (`self.PS`))
  (bind _asbp_bear (cast `/Game/Blueprints/Characters/Enemies/Bear/BP_Bear` (`self.GetOwningActorFromActorInfo`)))
  (`AbilitySystemComponent.TargetCancel` (`AbilitySystemBlueprintLibrary.GetAbilitySystemComponent` _asbp_bear))
  (`/Engine/EditorBlueprintResources/StandardMacros.IsValid` _ps
    (:`Is Valid`
      (`ActorComponent.K2_DestroyComponent` _ps))))