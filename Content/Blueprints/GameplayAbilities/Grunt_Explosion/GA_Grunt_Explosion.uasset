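; Gameplay ability for the Grunt that casts a targeted explosion, damaging and knocking back players.
; Activation starts user-confirmed targeting with BP_TargetActor while the cast montage plays.
; Valid target data spawns the explosion effect, then applies a damage effect and velocity-change impulse to each targeted player, before ending the ability.
; The impulse points away from the blast, rotated around the world right axis; ending the ability cancels targeting.
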(event `self.K2_ActivateAbility`
  (`self.K2_CommitAbility`)
  (bind (_asynctaskproxy _data) (`AbilityTask_WaitTargetData.WaitTargetData` "None" "UserConfirmed" "/Game/Blueprints/GameplayAbilities/Grunt_Explosion/BP_TargetActor.BP_TargetActor_C" (struct) (struct) null)
    (:`then`
      (`AbilityTask_PlayMontageAndWait.CreatePlayMontageAndWaitProxy` "None" "/Game/Blueprints/Characters/Enemies/Grunt/Animation/AM_Grunt_Cast.AM_Grunt_Cast"))
    (:`ValidData`
      (bind _returnvalue (`AbilitySystemBlueprintLibrary.GetTargetDataEndPoint` _data (- (`AbilitySystemBlueprintLibrary.GetDataCountFromTargetData` _data) 1)))
      (`GameplayStatics.SpawnEmitterAtLocation` "/Game/FXVarietyPack/Particles/P_ky_explosion.P_ky_explosion" _returnvalue (struct) (3.0 3.0 3.0))
      (for _array_element (`AbilitySystemBlueprintLibrary.GetActorsFromTargetData` _data)
        (bind _asbp_player (cast `/Game/Blueprints/Characters/Player/BP_Player` _array_element))
        (`self.ExplosionForce` _asbp_player _returnvalue 500.0)
        (`self.BP_ApplyGameplayEffectToTarget` (`AbilitySystemBlueprintLibrary.AbilityTargetDataFromActor` _asbp_player) "/Game/Blueprints/GameplayAbilities/Grunt_Explosion/Effect/GE_Grunt_Explosion_Damage.GE_Grunt_Explosion_Damage_C"))
      (`self.K2_EndAbility`))))

(event `self.K2_OnEndAbility`
  (params (bWasCancelled :type Boolean))
  (bind _asbp_grunt (cast `/Game/Blueprints/Characters/Enemies/Grunt/BP_Grunt` (`self.GetOwningActorFromActorInfo`)))
  (`AbilitySystemComponent.TargetCancel` (`RPGCharacter.AbilitySystemComp` _asbp_grunt)))

(fn `ExplosionForce`
  (params (Actor :type "Actor Object Reference") (Location :type "Vector Structure") (Magnitude :type "Float (double-precision)"))
  (bind _ascharacter (cast `Character` Actor))
  (`CharacterMovementComponent.AddImpulse` (`Character.CharacterMovement` _ascharacter) (`KismetMathLibrary.RotateAngleAxis` (* (`KismetMathLibrary.Normal` (- (`Actor.K2_GetActorLocation` _ascharacter) Location)) Magnitude) 30.0 (`KismetMathLibrary.Vector_Right`)) true))