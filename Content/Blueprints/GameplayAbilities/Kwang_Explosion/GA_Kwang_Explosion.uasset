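; Kwang's explosion gameplay ability: a player-aimed area blast that damages and knocks back targets and stuns enemies.
; Activation plays a cast montage in targeting mode and waits for confirmed target data from BP_ExplosionActor.
; On confirm it commits, plays a second montage, then spawns the delayed blast effect.
; ExplosionForce launches characters with a rotated outward impulse and physics-simulating actors radially; ending the ability resets targeting.
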(event `self.K2_ActivateAbility`
  (bind _result (`self.CanActivateAbility`))
  (if _result
    (bind _asbp_player (cast `/Game/Blueprints/Characters/Player/BP_Player` (`self.GetOwningActorFromActorInfo`)))
    (bind _asbp_player_controller (cast `/Game/Blueprints/BP_PlayerController` (`Pawn.GetController` _asbp_player)))
    (set `/Game/Blueprints/BP_PlayerController.isTargeting` true _asbp_player_controller)
    (`/Game/Blueprints/Characters/Player/BP_Player.ChangeRotationInput` _asbp_player true)
    (`AbilityTask_PlayMontageAndWait.CreatePlayMontageAndWaitProxy` "None" "/Game/Blueprints/GameplayAbilities/Kwang_Explosion/AnimationMontages/AM_Kwang_CastExplosion.AM_Kwang_CastExplosion"
      (:`then`
        (bind (_asynctaskproxy _data) (`AbilityTask_WaitTargetData.WaitTargetData` "None" "UserConfirmed" "/Game/Blueprints/GameplayAbilities/Kwang_Explosion/BP_ExplosionActor.BP_ExplosionActor_C" (struct) (struct) null)
          (:`ValidData`
            (`self.K2_CommitAbility`)
            (`self.PlayerActivateAbility`)
            (`AbilityTask_PlayMontageAndWait.CreatePlayMontageAndWaitProxy` "None" "/Game/Blueprints/GameplayAbilities/Kwang_Explosion/AnimationMontages/AM_Kwang_ExplosionConfirm.AM_Kwang_ExplosionConfirm"
              (:`then`
                (`KismetSystemLibrary.Delay` 0.5)
                (bind _returnvalue (`AbilitySystemBlueprintLibrary.GetTargetDataEndPoint` _data (- (`AbilitySystemBlueprintLibrary.GetDataCountFromTargetData` _data) 1)))
                (`GameplayStatics.SpawnEmitterAtLocation` "/Game/FXVarietyPack/Particles/P_ky_explosion.P_ky_explosion" _returnvalue)
                (for _array_element (`AbilitySystemBlueprintLibrary.GetActorsFromTargetData` _data)
                  (`self.ExplosionForce` _returnvalue 1000.0 _array_element)
                  (`self.BP_ApplyGameplayEffectToTarget` (`AbilitySystemBlueprintLibrary.AbilityTargetDataFromActor` _array_element) "/Game/Blueprints/GameplayAbilities/Kwang_Explosion/Effects/GE_Explosion_Damage.GE_Explosion_Damage_C")
                  (bind _asbp_enemy (cast `/Game/Blueprints/Characters/Enemies/BP_Enemy` _array_element))
                  (`/Game/Blueprints/Characters/Enemies/BP_Enemy.Stunt` _asbp_enemy 5.0))
                (`self.K2_EndAbility`)))))))
    (else
      (`self.K2_EndAbility`))))

(event `self.K2_OnEndAbility`
  (params (bWasCancelled :type Boolean))
  (bind _asbp_player (cast `/Game/Blueprints/Characters/Player/BP_Player` (`self.GetOwningActorFromActorInfo`)))
  (bind _asbp_player_controller (cast `/Game/Blueprints/BP_PlayerController` (`Pawn.GetController` _asbp_player)))
  (`/Game/Blueprints/Characters/Player/BP_Player.ChangeRotationInput` _asbp_player false)
  (set `/Game/Blueprints/BP_PlayerController.isTargeting` false _asbp_player_controller)
  (`AbilitySystemComponent.TargetCancel` (`RPGCharacter.AbilitySystemComp` _asbp_player)))

(fn `ExplosionForce`
  (params (CenterLocation :type "Vector Structure") (Magnitude :type "Float (double-precision)") (Actor :type "Actor Object Reference"))
  (bind _returnvalue (`Actor.GetComponentByClass` Actor "/Script/Engine.PrimitiveComponent"))
  (bind _ascharacter (cast `Character` Actor)
    (:`then`
      (`CharacterMovementComponent.AddImpulse` (`Character.CharacterMovement` _ascharacter) (`KismetMathLibrary.RotateAngleAxis` (* (`KismetMathLibrary.Normal` (- (`Actor.K2_GetActorLocation` _ascharacter) CenterLocation)) Magnitude) 30.0 (`KismetMathLibrary.Vector_Right`)) true))
    (:`CastFailed`
      (if (`SceneComponent.IsSimulatingPhysics` _returnvalue "None")
        (`PrimitiveComponent.AddRadialImpulse` _returnvalue CenterLocation 200.0 Magnitude "RIF_Constant" true)))))