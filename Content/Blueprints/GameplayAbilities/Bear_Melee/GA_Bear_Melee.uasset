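; Gameplay ability for the bear enemy's melee attack, played with fire effects on both of its weapons.
; On activation it commits, attaches fireball particles to the left and right weapons and plays the attack montage.
; A Bear.melee.damage gameplay event launches the payload's target via PushCharacter and applies the melee damage effect to it.
; The ability ends when the montage finishes or is interrupted, destroying both particle components.
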(event `self.K2_ActivateAbility`
  (`self.K2_CommitAbility`)
  (bind _asbp_bear (cast `/Game/Blueprints/Characters/Enemies/Bear/BP_Bear` (`self.GetOwningActorFromActorInfo`)))
  (bind _returnvalue (`GameplayStatics.SpawnEmitterAttached` "/Game/FXVarietyPack/Particles/P_ky_fireBall.P_ky_fireBall" (`/Game/Blueprints/Characters/Enemies/Bear/BP_Bear.Weapon_L` _asbp_bear)))
  (set `self.F1` _returnvalue)
  (bind _returnvalue_2 (`GameplayStatics.SpawnEmitterAttached` "/Game/FXVarietyPack/Particles/P_ky_fireBall.P_ky_fireBall" (`/Game/Blueprints/Characters/Enemies/Bear/BP_Bear.Weapon_R` _asbp_bear)))
  (set `self.F2` _returnvalue_2)
  (`AbilityTask_PlayMontageAndWait.CreatePlayMontageAndWaitProxy` "None" "/Game/Blueprints/Characters/Enemies/Bear/Animation/AM_Bear_AttackSimple.AM_Bear_AttackSimple"
    (:`then`
      (bind (_asynctaskproxy _payload) (`AbilityTask_WaitGameplayEvent.WaitGameplayEvent` (struct :`TagName` "bear.melee.damage") null)
        (:`EventReceived`
          (bind _asbp_enemy (cast `/Game/Blueprints/Characters/Enemies/BP_Enemy` (`self.GetOwningActorFromActorInfo`)))
          (`RPGCharacter.PushCharacter` _asbp_enemy (`.Target` (break `GameplayEventData` _payload)) 20.0 3000.0)
          (`self.BP_ApplyGameplayEffectToTarget` (`AbilitySystemBlueprintLibrary.AbilityTargetDataFromActor` (`.Target` (break `GameplayEventData` _payload))) "/Game/Blueprints/GameplayAbilities/Bear_Melee/Effects/GE_Bear_Melee_Damage.GE_Bear_Melee_Damage_C"))))
    (:`OnCompleted`
      (`self.K2_EndAbility` :!label _label))
    (:`OnBlendOut`
      (goto _label))
    (:`OnInterrupted`
      (goto _label))
    (:`OnCancelled`
      (goto _label))))

(event `self.K2_OnEndAbility`
  (params (bWasCancelled :type Boolean))
  (`ActorComponent.K2_DestroyComponent` (`self.F1`))
  (`ActorComponent.K2_DestroyComponent` (`self.F2`)))