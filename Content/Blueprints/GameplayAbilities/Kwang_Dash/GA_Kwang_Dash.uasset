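; Kwang's dash gameplay ability, which launches a grounded player forward through pawns and damages those reported as hit.
; Activation commits, turns on the zoom flag, attaches a lightning effect, switches capsule Pawn collision to Overlap and applies a forward velocity-change impulse.
; It applies GE_Dash_Damage to targets from Skill.dash.dealDamage gameplay events during the brief dash window.
; After a short delay it clears zoom and ends, restoring Pawn blocking.
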(event `self.K2_ActivateAbility`
  (bind _result (`self.CanActivateAbility`))
  (if _result
    (bind _asbp_player (cast `/Game/Blueprints/Characters/Player/BP_Player` (`self.GetOwningActorFromActorInfo`)))
    (if (not (`NavMovementComponent.IsFalling` (`Character.CharacterMovement` _asbp_player)))
      (`self.K2_CommitAbility`)
      (bind _asbp_player_2 (cast `/Game/Blueprints/Characters/Player/BP_Player` (`self.GetOwningActorFromActorInfo`)))
      (set `RPGCharacter.bWantsToZoom` true _asbp_player_2)
      (`GameplayStatics.SpawnEmitterAttached` "/Game/FXVarietyPack/Particles/P_ky_lightning2.P_ky_lightning2" (`Actor.RootComponent` _asbp_player_2) "None" (0.0 0.0 -50.0))
      (`self.Dash` 20000.0)
      (bind (_asynctaskproxy _payload) (`AbilityTask_WaitGameplayEvent.WaitGameplayEvent` (struct :`TagName` "skill.dash.dealDamage") null)
        (:`then`
          (`KismetSystemLibrary.Delay` 0.2)
          (set `RPGCharacter.bWantsToZoom` false _asbp_player_2)
          (`self.K2_EndAbility`))
        (:`EventReceived`
          (`self.BP_ApplyGameplayEffectToTarget` (`AbilitySystemBlueprintLibrary.AbilityTargetDataFromActor` (`.Target` (break `GameplayEventData` _payload))) "/Game/Blueprints/GameplayAbilities/Kwang_Dash/Effects/GE_Dash_Damage.GE_Dash_Damage_C"))))))

(event `self.K2_OnEndAbility`
  (params (bWasCancelled :type Boolean))
  (bind _asbp_player (cast `/Game/Blueprints/Characters/Player/BP_Player` (`self.GetOwningActorFromActorInfo`)))
  (`PrimitiveComponent.SetCollisionResponseToChannel` (`Character.CapsuleComponent` _asbp_player) "ECC_Pawn" "ECR_Block"))

(fn `Dash`
  (params (Speed :type "Float (double-precision)"))
  (bind _returnvalue (`self.GetOwningActorFromActorInfo`))
  (bind _asbp_player (cast `/Game/Blueprints/Characters/Player/BP_Player` _returnvalue))
  (`PrimitiveComponent.SetCollisionResponseToChannel` (`Character.CapsuleComponent` _asbp_player) "ECC_Pawn" "ECR_Overlap")
  (`CharacterMovementComponent.AddImpulse` (`Character.CharacterMovement` _asbp_player) (* (`Actor.GetActorForwardVector` _returnvalue) Speed) true))