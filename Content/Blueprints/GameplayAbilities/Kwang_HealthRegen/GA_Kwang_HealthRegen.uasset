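; Gameplay ability for Kwang's self-heal, which ends without committing if activation is not allowed or health is already at max.
; Current and max health come from the owner's attribute set, fetched via a message call.
; After committing, it starts the heal montage and immediately spawns attached sound and aura particles and applies the health regen GameplayEffect to the owner.
; The ability ends when the montage completes, blends out, or is interrupted or cancelled.
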(event `self.K2_ActivateAbility`
  (bind _rootcomponent (`Actor.RootComponent` (`self.GetOwningActorFromActorInfo`)))
  (bind _result (`self.CanActivateAbility`))
  (if _result
    (bind _returnvalue (message `RPGAttributeSetInterface.GetAttributeSetComp` (`self.GetOwningActorFromActorInfo`)))
    (bind (_health_basevalue _health_currentvalue) (break `GameplayAttributeData` (`RPGAttributeSet.Health` _returnvalue)))
    (bind (_maxhealth_basevalue _maxhealth_currentvalue) (break `GameplayAttributeData` (`RPGAttributeSet.MaxHealth` _returnvalue)))
    (if (== _health_currentvalue _maxhealth_currentvalue)
      (`self.K2_EndAbility` :!label _label)
      (else
        (`self.K2_CommitAbility`)
        (`AbilityTask_PlayMontageAndWait.CreatePlayMontageAndWaitProxy` "None" "/Game/Blueprints/GameplayAbilities/Kwang_HealthRegen/AnimMontages/AM_Kwang_HealthRegen.AM_Kwang_HealthRegen"
          (:`then`
            (`GameplayStatics.SpawnSoundAttached` "/Game/Blueprints/GameplayAbilities/Kwang_HealthRegen/Sound/HealthRegenSound.HealthRegenSound" _rootcomponent "None" (0.0 0.0 0.0) (struct) "KeepRelativeOffset" false 1.0 1.0 0.0 null null)
            (`GameplayStatics.SpawnEmitterAttached` "/Game/FXVarietyPack/Particles/P_ky_healAura.P_ky_healAura" _rootcomponent "None" (0.0 0.0 -50.0))
            (`self.BP_ApplyGameplayEffectToOwner` "/Game/Blueprints/GameplayAbilities/Kwang_HealthRegen/Effects/GE_HealthRegen_Amount.GE_HealthRegen_Amount_C"))
          (:`OnCompleted`
            (`self.K2_EndAbility` :!label _label_2))
          (:`OnBlendOut`
            (goto _label_2))
          (:`OnInterrupted`
            (goto _label_2))
          (:`OnCancelled`
            (goto _label_2)))))
    (else
      (goto _label))))